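; BP_MyPlayer is a player actor Blueprint that throws grenades and reacts to damage.
; A right mouse click spawns a BP_Grenade at the GrenadeDir component's world transform, adjusting for collisions but always spawning.
; AnyDamage only prints the damage amount as an "Ouch" debug string, with no health handling.
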(event `Key|RightMouseButton`
  (params (Key :type "Key Structure"))
  ;[1 1 1] On spawn un grenade au Clic Droit
  (:`Pressed`
    (`|SpawnActorFromClass` "/Game/MyContent/Actors/BP_Grenade.BP_Grenade_C" (`SceneComponent.K2_GetComponentToWorld` (`self.GrenadeDir`)) "AdjustIfPossibleButAlwaysSpawn" "MultiplyWithRoot" null null)))

(event `self.ReceiveAnyDamage`
  (params (Damage :type "Float (single-precision)") (DamageType :type "DamageType Object Reference") (InstigatedBy :type "Controller Object Reference") (DamageCauser :type "Actor Object Reference"))
  ;[1 1 1] Réception des dégâts
  (`KismetSystemLibrary.PrintString` (`KismetStringLibrary.Concat_StrStr` "Ouch !!!! => " (`KismetStringLibrary.Conv_DoubleToString` Damage))))

(fn `UserConstructionScript`
  (`parent.UserConstructionScript`))