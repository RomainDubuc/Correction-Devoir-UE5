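; Timed grenade actor that blinks faster and faster, then explodes, damaging nearby Characters.
; After an initial delay, a self-calling BlinkOnce event swaps the sphere material, using a quadratic ease-out to shorten each interval.
; Overlapping a Character also detonates it once a brief arming time, tracked in Tick, has passed.
; Detonation plays sound and particles, applies damage through a debug-drawn multi-sphere trace, then destroys the actor.
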(event `self.ReceiveBeginPlay`
  ;[1 1 1] Après un temps défini, démarre son Clignottement avant explosion.
  (set `self.BaseMaterial` (`PrimitiveComponent.GetMaterial` (`self.Sphere`) 0))
  (`KismetSystemLibrary.Delay` (`self.WaitDuration`))
  (set `self.CurrentBlink` 0)
  (`self.BlinkOnce`))

(event `BlinkOnce`
  ;[1 1 1] Accomplit un Blink après un temps défini de plus en plus court. L'Event se rappelle en boucle jusqu'à NbBlinks appels successifs. Explose à la fin.
  (bind _res (`/Game/MyContent/Lib_Ease.EaseQuadOut` (* (`KismetMathLibrary.Conv_IntToDouble` (`self.CurrentBlink`)) (/ 1.0 (`KismetMathLibrary.Conv_IntToDouble` (`self.NbBlinks`)))))) ; Permet d'avoir un delta très gros au début et très petit sur la fin.
  (`KismetSystemLibrary.Delay` (- (`self.BlinkMaxDuration`) (* _res (`self.BlinkMaxDuration`))))
  (`PrimitiveComponent.SetMaterial` (`self.Sphere`) 0 (`self.BlinkMaterial`))
  (`KismetSystemLibrary.Delay` 0.1)
  (`PrimitiveComponent.SetMaterial` (`self.Sphere`) 0 (`self.BaseMaterial`))
  (bind _result (`/Engine/EditorBlueprintResources/StandardMacros.IncrementInt` (`self.CurrentBlink`))
    (:`  `
      (if (< _result (`self.NbBlinks`))
        (`self.BlinkOnce`)
        (else
          (`self.AutoDestroy`))))))

(event `AutoDestroy`
  ;[1 1 1] Gère la destruction de la Grenade
  (`GameplayStatics.PlaySound2D` "/Game/StarterContent/Audio/Explosion01.Explosion01" 1.0 1.0 0.0 null null)
  (`GameplayStatics.SpawnEmitterAtLocation` "/Game/StarterContent/Particles/P_Explosion.P_Explosion" (`self.K2_GetActorLocation`))
  (`self.GenerateDamages`)
  (`self.K2_DestroyActor`))

(event `self.ReceiveActorBeginOverlap`
  (params (OtherActor :type "Actor Object Reference"))
  ;[1 1 1] Active la destruction de la Grenade au moindre contact avec un Character
  (if (> (`self.LifeTime`) 0.25)
    (cast `Character` OtherActor)
    (`self.AutoDestroy`)))

(event `self.ReceiveTick`
  (params (DeltaSeconds :type "Float (single-precision)"))
  ;[1 1 1] Gère le temps de vie de la Grenade
  (set `self.LifeTime` (+ DeltaSeconds (`self.LifeTime`))))

(event `GenerateDamages`
  (bind _returnvalue (`self.K2_GetActorLocation`))
  ;[1 1 1] Application des dégâts aux Actors concernés
  (bind _outhits (`KismetSystemLibrary.SphereTraceMulti` :`Start` _returnvalue :`End` _returnvalue :`Radius` 500.0 :`TraceChannel` "TraceTypeQuery3" :`DrawDebugType` "ForDuration" :`DrawTime` 2.0))
  (for _array_element _outhits
    (bind _ascharacter (cast `Character` (`.HitActor` (`GameplayStatics.BreakHitResult` _array_element))))
    (`GameplayStatics.ApplyDamage` _ascharacter (`KismetMathLibrary.Conv_IntToDouble` (`self.DamagePower`)) null self)))

(fn `UserConstructionScript`)