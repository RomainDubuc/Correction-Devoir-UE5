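; BP_EndLEvel is a collectible that ends the level when picked up.
; Its pickup prompt widget starts hidden and is toggled through SetWidgetVisibility, while Tick bobs the sphere mesh with a cosine of accumulated time.
; PickUp hides the prompt and actor, spawns a scaled-down explosion, then after a short delay adds the UI_EndLevel widget to the viewport and destroys the actor.
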(event `SetWidgetVisibility`
  (params (canShow :type Boolean))
  ;[1 0.9492 0] Gestion du Widget pour ramasser l'item
  (`SceneComponent.SetVisibility` (`self.WidgetPickUp`) canShow false))

(event `self.ReceiveBeginPlay`
  ;[1 0.9492 0] Gestion du Widget pour ramasser l'item
  (`self.SetWidgetVisibility` false) ; Le Widget démarre invisble
)

(event `self.ReceiveTick`
  (params (DeltaSeconds :type "Float (single-precision)"))
  ;[0 0.2653 1] Ajout d'un effet de flotaison sur le Collectible
  (bind _output_get (set `self.totalTime` (+ DeltaSeconds (`self.totalTime`))))
  (`SceneComponent.K2_AddLocalOffset` (`self.MeshSphere`) (`KismetMathLibrary.MakeVector` 0.0 0.0 (* (`KismetMathLibrary.Cos` _output_get) 0.1)) false false))

(event `PickUp`
  ;[0 1 0.2294] Déclenche la fin du niveau
  (`self.SetWidgetVisibility` false)
  (bind _returnvalue (`GameplayStatics.SpawnEmitterAtLocation` "/Game/StarterContent/Particles/P_Explosion.P_Explosion" (`self.K2_GetActorLocation`)))
  (`SceneComponent.SetRelativeScale3D` _returnvalue (0.1 0.1 0.1))
  (`self.SetActorHiddenInGame` true)
  (`KismetSystemLibrary.Delay` 1.0)
  (bind _returnvalue_2 (`|CreateWidget` "/Game/MyContent/UI/Menus/UI_EndLevel.UI_EndLevel_C"))
  (`UserWidget.AddToViewport` _returnvalue_2 0)
  (`self.K2_DestroyActor`))

(fn `UserConstructionScript`)