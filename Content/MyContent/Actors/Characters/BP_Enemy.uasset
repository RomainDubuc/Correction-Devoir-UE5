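; BP_Enemy is an enemy character that takes damage, shows a health bar and explodes when killed.
; BeginPlay caches the mesh's default material, fills HP and gets the progress bar from its UI_Enemy widget component.
; AnyDamage clamps HP, then either briefly flashes the mesh material using a retriggerable delay or spawns an explosion and destroys the actor.
; Tick refreshes the bar every frame, showing it only below full health.
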(event `self.ReceiveBeginPlay`
  ;[1 1 1] Initialisation de l'Ennemi
  (set `self.DefaultMaterial` (`PrimitiveComponent.GetMaterial` (`self.Mesh`) 1))
  (set `self.CurrentHP` (`self.MaxHP`))
  (bind _asui_enemy (cast `/Game/MyContent/UI/UI/UI_Enemy` (`WidgetComponent.GetWidget` (`self.UI_HP_Component`))))
  (set `self.HP Progress Bar` (`/Game/MyContent/UI/UI/UI_Enemy.HP_ProgressBar` _asui_enemy)))

(event `self.ReceiveAnyDamage`
  (params (Damage :type "Float (single-precision)") (DamageType :type "DamageType Object Reference") (InstigatedBy :type "Controller Object Reference") (DamageCauser :type "Actor Object Reference"))
  ;[1 1 1] Réception des dégâts et mort
  (bind _output_get (set `self.CurrentHP` (`KismetMathLibrary.FClamp` (- (`self.CurrentHP`) Damage) 0.0 (`self.MaxHP`))))
  (if (> _output_get 0.0)
    (`PrimitiveComponent.SetMaterial` (`self.Mesh`) 1 "/Engine/MapTemplates/Materials/BasicTemplateMaterial.BasicTemplateMaterial")
    (`KismetSystemLibrary.RetriggerableDelay` 0.1)
    (`PrimitiveComponent.SetMaterial` (`self.Mesh`) 1 (`self.DefaultMaterial`))
    (else
      (`GameplayStatics.SpawnEmitterAtLocation` "/Game/StarterContent/Particles/P_Explosion.P_Explosion" (`self.K2_GetActorLocation`))
      (`self.K2_DestroyActor`))))

(event `self.ReceiveTick`
  (params (DeltaSeconds :type "Float (single-precision)"))
  (bind _hp_progress_bar (`self.HP Progress Bar`))
  ;[1 1 1] On gère la Barre d'HP suivant les HP actuels
  (`ProgressBar.SetPercent` (`self.HP Progress Bar`) (/ (`self.CurrentHP`) (`self.MaxHP`)))
  (if (< (`self.CurrentHP`) (`self.MaxHP`))
    (set `Widget.Visibility` "Visible" _hp_progress_bar)
    (else
      (set `Widget.Visibility` "Hidden" _hp_progress_bar))))

(fn `UserConstructionScript`)