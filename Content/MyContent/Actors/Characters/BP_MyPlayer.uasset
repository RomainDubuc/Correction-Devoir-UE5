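; Player character Blueprint handling shooting, grenades, health, item pickup and death.
; On BeginPlay it creates the HUD and runs an intro camera sweep: detached camera, tick-recursive smoothstep to a level target and back, input disabled.
; Held fire repeats line traces on a delay; a timeline drives gold-material invincibility and its bar.
; Damage blinks the mesh or triggers Game Over; landing damage scales from tracked airborne peak Z.
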(event `self.ReceiveBeginPlay`
  (bind _returnvalue (`GameplayStatics.GetPlayerController` 0))
  ;[0.07239 0.6204 1] Initialisation des éléments de base
  (`parent.ReceiveBeginPlay`)
  (set `self.DefaultMaterialIn` (`PrimitiveComponent.GetMaterial` (`self.Mesh`) 0))
  (set `self.DefaultMaterialOut` (`PrimitiveComponent.GetMaterial` (`self.Mesh`) 1))
  (bind _returnvalue_2 (`|CreateWidget` "/Game/MyContent/UI/UI/UI_Player.UI_Player_C"))
  (bind _output_get (set `self.UI` _returnvalue_2))
  (`UserWidget.AddToViewport` _output_get 0)
  (set `Widget.Visibility` "Hidden" (`/Game/MyContent/UI/UI/UI_Player.Inv_ProgressBar` _output_get))
  (set `PlayerController.bShowMouseCursor` false _returnvalue)
  (`WidgetBlueprintLibrary.SetInputMode_GameOnly` _returnvalue)
  (set `self.CurrentHP` (`self.MaxHP`))
  (`self.StartCameraEvent`))

(event `StartCameraEvent`
  (bind _followcamera (`self.FollowCamera`))
  ;[0.3371 1 0.5028] Event de Caméra
  ;;[1 1 1] Démarre l'Event de Caméra
  (`SceneComponent.K2_AttachToComponent` (`self.FollowCamera`) null "None" "KeepWorld" "KeepWorld" "KeepWorld" true) ; On retire la Caméra de CameraBoom afin de pouvoir la manipuler
  (set `self.CameraStartPosition` (`SceneComponent.K2_GetComponentLocation` _followcamera))
  (set `self.CameraStartRotation` (`SceneComponent.K2_GetComponentRotation` _followcamera))
  (bind _returnvalue (`GameplayStatics.GetActorOfClass` "/Game/MyContent/Actors/Others/BP_CameraTargetCutscene.BP_CameraTargetCutscene_C")) ; On récupère l'Actor placé sur le niveau qui défini la Position et Rotation cible de la Caméra
  (set `self.CameraMoveBy` (- (`self.K2_GetActorLocation` _returnvalue) (`self.CameraStartPosition`)))
  (set `self.CameraRotateBy` (`KismetMathLibrary.ComposeRotators` (`self.K2_GetActorRotation` _returnvalue) (* (`self.CameraStartRotation`) -1.0)))
  (`self.DisableInput` (`GameplayStatics.GetPlayerController` 0)) ; On retire les contrôles au joueur.
  (`KismetSystemLibrary.Delay` 2.0)
  (`self.CameraEventLoop` 0.0 1.0))

(event `CameraEventLoop`
  (params (timer :type "Float (double-precision)") (direction :type "Float (double-precision)"))
  ;[0.3371 1 0.5028] Event de Caméra
  ;;[1 1 1] Effectue un Step dans le déplacement de la Caméra
  (`KismetSystemLibrary.DelayUntilNextTick`)
  (bind _timeratio (`self.AddDeltaTimeRatio` timer direction 4.0))
  (bind (_newposition _newrotation) (`self.GetNewCameraPosAndRot` _timeratio)) ; On obtient la nouvelle Position et Rotation à donner à la Caméra
  (`SceneComponent.K2_SetWorldLocationAndRotation` (`self.FollowCamera`) _newposition _newrotation false false)
  (bind _returnvalue (`self.IsBetween` _timeratio 0.0 1.0)) ; On check si le Timer n'a pas dépassé 0 ou 1
  (if _returnvalue
    (`self.CameraEventLoop` _timeratio direction) ; On continue dans la Direction actuelle
    (elif (< direction 0.0)
      (`SceneComponent.K2_AttachToComponent` (`self.FollowCamera`) (`self.CameraBoom`) "None" "KeepWorld" "KeepWorld" "KeepWorld" true) ; On replace la Caméra dans CameraBoom
      (`self.EnableInput` (`GameplayStatics.GetPlayerController` 0))
      (else
        (`KismetSystemLibrary.Delay` 1.0)
        (`self.CameraEventLoop` 1.0 -1.0) ; On Inverse la Direction \net on fait le mouvement inverse après un temps de pause
      ))))

(event `Key|RightMouseButton`
  (params (Key :type "Key Structure"))
  ;[1 0.1458 0.1557] Armement et Attaques
  ;;[1 1 1] On spawn un grenade au Clic Droit
  (:`Pressed`
    (`|SpawnActorFromClass` "/Game/MyContent/Actors/Projectiles/BP_Grenade.BP_Grenade_C" (`SceneComponent.K2_GetComponentToWorld` (`self.GrenadeDir`)) "AdjustIfPossibleButAlwaysSpawn" "MultiplyWithRoot" null null)))

(event `Key|LeftMouseButton`
  (params (Key :type "Key Structure"))
  ;[1 0.1458 0.1557] Armement et Attaques
  ;;[1 1 1] Déclenche le Tir en rafale et conditionne son arrêt
  (:`Pressed`
    (set `self.ShootKeyPressed` true)
    (`self.ShootEventLoop`))
  (:`Released`
    (set `self.ShootKeyPressed` false)))

(event `ShootEventLoop`
  (bind _shootdir (`self.ShootDir`))
  (bind _returnvalue (`SceneComponent.K2_GetComponentLocation` _shootdir))
  ;[1 0.1458 0.1557] Armement et Attaques
  ;;[1 1 1] Gestion du Tir en Rafale, s'auto rappelle tant que la touche de Tir est maintenue.
  (bind _outhit (`KismetSystemLibrary.LineTraceSingle` :`Start` _returnvalue :`End` (+ _returnvalue (* (`SceneComponent.GetForwardVector` _shootdir) (`self.ShootDistanceMax`))) :`TraceChannel` "TraceTypeQuery3" :`DrawDebugType` "ForDuration" :`DrawTime` (/ (`self.ShootDelay`) 2.0)))
  (bind _asbp_enemy (cast `/Game/MyContent/Actors/Characters/BP_Enemy` (`.HitActor` (`GameplayStatics.BreakHitResult` _outhit))))
  (`GameplayStatics.ApplyDamage` _asbp_enemy (`self.ShootPower`) null self)
  (`KismetSystemLibrary.Delay` (`self.ShootDelay`))
  (if (`self.ShootKeyPressed`)
    (`self.ShootEventLoop`)))

(event `StartInvincibility`
  ;[0.9084 0.09994 1] Déclenche et gère l'invincibilité du joueur
  (set `Widget.Visibility` "Visible" (`/Game/MyContent/UI/UI/UI_Player.Inv_ProgressBar` (`self.UI`))) ; On affiche la barre
  (set `self.IsInvincible` true)
  (`PrimitiveComponent.SetMaterial` (`self.Mesh`) 0 "/Game/StarterContent/Materials/M_Metal_Gold.M_Metal_Gold")
  (bind (_direction _remaininginvincibilitytime) (`Timeline|InvincibilityTime` :!via `PlayFromStart`) ; On déclenche PlayFromStart pour que, si l'on ramasse encore l'Item, ça redémarre depuis le début
    (:`Update`
      (bind _res (`/Game/MyContent/Libraries/Lib_Ease.EaseQuadOut` _remaininginvincibilitytime)) ; Permet de modifier un peu l'affichage de la barre afin qu'elle passe un peu plus de temps en étant presque vide
      (`ProgressBar.SetPercent` (`/Game/MyContent/UI/UI/UI_Player.Inv_ProgressBar` (`self.UI`)) (- 1.0 _res)))
    (:`Finished`
      (set `self.IsInvincible` false)
      (`PrimitiveComponent.SetMaterial` (`self.Mesh`) 0 (`self.DefaultMaterialIn`))
      (set `Widget.Visibility` "Hidden" (`/Game/MyContent/UI/UI/UI_Player.Inv_ProgressBar` (`self.UI`))) ; On cache la barre
    )))

(event `Key|E`
  (params (Key :type "Key Structure"))
  ;[0 0.08263 1] Gestion des Items ramassable avec la touche E (et de leur Widget)
  (:`Pressed`
    (`/Engine/EditorBlueprintResources/StandardMacros.IsValid` (`self.InterractableItem`)
      (:`Is Valid`
        (`/Game/MyContent/Actors/Collectibles/BP_EndLEvel.PickUp` (`self.InterractableItem`))
        (set `self.InterractableItem` null)))))

(event `self.ReceiveTick`
  (params (DeltaSeconds :type "Float (single-precision)"))
  ;[1 0.7745 0] Dégâts et Mort
  ;;[1 1 1] S'exécute à chaque Frame
  (`ProgressBar.SetPercent` (`/Game/MyContent/UI/UI/UI_Player.HP_ProgressBar` (`self.UI`)) (/ (`self.CurrentHP`) (`self.MaxHP`))) ; Mise à jour de la Barre d'HP
  (`self.Update Aerian Peak`) ; Maj de la position du chute max
)

(event `self.ReceiveActorBeginOverlap`
  (params (OtherActor :type "Actor Object Reference"))
  ;[0 0.08263 1] Gestion des Items ramassable avec la touche E (et de leur Widget)
  (bind _asbp_end_level (cast `/Game/MyContent/Actors/Collectibles/BP_EndLEvel` OtherActor))
  (bind _output_get (set `self.InterractableItem` _asbp_end_level))
  (`/Game/MyContent/Actors/Collectibles/BP_EndLEvel.SetWidgetVisibility` _output_get true))

(event `self.ReceiveActorEndOverlap`
  (params (OtherActor :type "Actor Object Reference"))
  ;[0 0.08263 1] Gestion des Items ramassable avec la touche E (et de leur Widget)
  (bind _asbp_end_level (cast `/Game/MyContent/Actors/Collectibles/BP_EndLEvel` OtherActor))
  (`/Game/MyContent/Actors/Collectibles/BP_EndLEvel.SetWidgetVisibility` _asbp_end_level false)
  (set `self.InterractableItem` null))

(event `self.ReceiveAnyDamage`
  (params (Damage :type "Float (single-precision)") (DamageType :type "DamageType Object Reference") (InstigatedBy :type "Controller Object Reference") (DamageCauser :type "Actor Object Reference"))
  ;[1 0.7745 0] Dégâts et Mort
  ;;[1 1 1] Réception des dégâts
  (if (not (`self.IsInvincible`))
    (bind _output_get (set `self.CurrentHP` (`KismetMathLibrary.FClamp` (- (`self.CurrentHP`) Damage) 0.0 (`self.MaxHP`))))
    (if (<= _output_get 0.0)
      (`self.LaunchDeath`)
      (else
        (`self.BlinkDamage`)))))

(event `BlinkDamage`
  ;[1 0.7745 0] Dégâts et Mort
  ;;[1 1 1] Blink de réception de dégâts
  (`PrimitiveComponent.SetMaterial` (`self.Mesh`) 1 "/Engine/MapTemplates/Materials/BasicTemplateMaterial.BasicTemplateMaterial")
  (`KismetSystemLibrary.RetriggerableDelay` 0.1)
  (`PrimitiveComponent.SetMaterial` (`self.Mesh`) 1 (`self.DefaultMaterialOut`)))

(event `LaunchDeath`
  (bind _returnvalue (`GameplayStatics.GetPlayerController` 0))
  ;[1 0.7745 0] Dégâts et Mort
  ;;[1 1 1] Gère la Mort du Joueur
  (`GameplayStatics.SpawnEmitterAtLocation` "/Game/StarterContent/Particles/P_Explosion.P_Explosion" (`self.K2_GetActorLocation`))
  (`self.SetActorHiddenInGame` true)
  (`self.DisableInput` _returnvalue)
  (`KismetSystemLibrary.Delay` 0.5)
  (bind _returnvalue_2 (`|CreateWidget` "/Game/MyContent/UI/Menus/UI_GameOver.UI_GameOver_C" _returnvalue))
  (`UserWidget.AddToViewport` _returnvalue_2 0))

(event `self.OnLanded`
  (params (Hit :type "HitResult Structure (by ref)"))
  (bind (_returnvalue_x _returnvalue_y _returnvalue_z) (`KismetMathLibrary.BreakVector` (`self.K2_GetActorLocation`)))
  ;[1 0.7745 0] Dégâts et Mort
  ;;[1 1 1] Dégâts de Chute
  (if (> (`self.MaxFallPosZ`) (`self.FallDistanceForDamages`))
    (`GameplayStatics.ApplyDamage` self (`KismetMathLibrary.MapRangeClamped` (- (`self.MaxFallPosZ`) _returnvalue_z) (`self.FallDistanceForDamages`) 1000.0 10.0 30.0))))

(fn `AddDeltaTimeRatio`
  (params (OldVal :type "Float (double-precision)") (Direction :type "Float (double-precision)") (Duration :type "Float (double-precision)"))
  (returns (TimeRatio :type "Float (double-precision)"))
  ;[1 1 1] Ajoute ou retire, suivant Direction, à OldVal le temps écoulé depuis la dernière frame divisé par le temps total voulu afin d'avoir une valeur de retour entre 0 et 1.
  (return (+ OldVal (/ (* Direction (`GameplayStatics.GetWorldDeltaSeconds`)) Duration))))

(fn `GetNewCameraPosAndRot`
  (params (CurrentTimer :type "Float (double-precision)"))
  (returns (NewPosition :type "Vector Structure") (NewRotation :type "Rotator Structure"))
  ;[1 1 1] Renvoie la nouvelle Position et la nouvelle Rotation de la Caméra à partir de CurrentTime, en adoucissant les mouvements sur les extrêmités.
  (bind _res (`/Game/MyContent/Libraries/Lib_Ease.Smoothstep` CurrentTimer)) ; On passe le timer dans une fonction Ease pour adoucir les mouvements sur les bords
  (return (+ (* (`self.CameraMoveBy`) _res) (`self.CameraStartPosition`)) (`KismetMathLibrary.ComposeRotators` (`self.CameraStartRotation`) (* (`self.CameraRotateBy`) _res))))

(fn `IsBetween`
  (params (val :type "Float (double-precision)") (min :type "Float (double-precision)") (max :type "Float (double-precision)"))
  (returns (ReturnValue :type Boolean))
  ;[1 1 1] Renvoie True si Val est compris entre Min et Max (non inclus)
  (return (and (> val min) (< val max))))

(fn `Update Aerian Peak`
  (bind (_returnvalue_x _returnvalue_y _returnvalue_z) (`KismetMathLibrary.BreakVector` (`self.K2_GetActorLocation`)))
  ;[1 1 1] Met à jour la variable MaxFallPosZ qui contient la position Z maximale atteinte durant le saut / la chute
  (if (`NavMovementComponent.IsFalling` (`self.CharacterMovement`))
    (set `self.MaxFallPosZ` (`KismetMathLibrary.FMax` (`self.MaxFallPosZ`) _returnvalue_z))
    (else
      (set `self.MaxFallPosZ` 0.0))))

(fn `UserConstructionScript`
  (`parent.UserConstructionScript`))