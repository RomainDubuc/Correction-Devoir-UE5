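; Moving platform actor that shuttles its Cube back and forth along a spline.
; Tick calls StepMove to advance normalized time over the spline's Duration, then samples the location through Smoothstep to ease both ends.
; At each end it either pauses for WaitOnCorners, stops under StopAtEnd until a BP_MyPlayer overlap (also its initial state), or reverses immediately.
; Immediate reversals reflect overshoot instead of clamping, keeping multiple platforms in sync.
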(event `self.ReceiveBeginPlay`
  ;[1 1 1] Si la PF est en mode StopAtEnd, elle démarre arrêtée.
  (if (`self.stopAtEnd`)
    (set `self.stopped` true)))

(event `self.ReceiveActorBeginOverlap`
  (params (OtherActor :type "Actor Object Reference"))
  ;[1 1 1] Si un Player monte sur la Plateforme et qu'elle est stoppée, on enlève le Stop.
  (cast `/Game/MyContent/Actors/BP_MyPlayer` OtherActor)
  (set `self.stopped` false))

(event `self.ReceiveTick`
  (params (DeltaSeconds :type "Float (single-precision)"))
  ;[1 1 1] A chaque frame, on met à jour l'état du déplacement de la Plateforme sur le Spline et on la positionne là où elle doit être.
  (if (not (`self.stopped`))
    (`self.StepMove` DeltaSeconds) ; Ceci met à jour l'état du déplacement
    (bind _res (`/Game/MyContent/Lib_Ease.Smoothstep` (`self.tmpTime`))) ; On passe tmpTime dans un SmoothStep pour adoucir les déplacements sur les bords.
    (`SceneComponent.K2_SetRelativeLocationAndRotation` (`self.Cube`) (.location (`SplineComponent.GetTransformAtTime` (`self.Spline`) (* _res (`SplineComponent.Duration` (`self.Spline`))) "Local" true false)) (`KismetMathLibrary.MakeRotator` 0.0) false false) ; On positionne la PF à l'endroit où elle doit être sur le Spline
  ))

(fn `DoStepTime`
  (params (dt :type "Float (double-precision)"))
  ;[1 1 1] On met à jour tmpTime suivant le temps écoulé à chaque frame et la direction de déplacement
  (set `self.tmpTime` (+ (`self.tmpTime`) (/ (* dt (`self.moveDirection`)) (`SplineComponent.Duration` (`self.Spline`)))))
  (return))

(fn `DoWaitStep`
  (params (dt :type "Float (double-precision)"))
  (returns (mustWait :type Boolean))
  ;[1 1 1] Met à jour CurrentWait suivant le temps écoulé et renvoie True si la Plateforme doit encore attendre, Faux sinon.
  (bind _output_get (set `self.currentWait` (- (`self.currentWait`) dt)))
  (return (> _output_get 0.0)))

(fn `IsWaitOrStop`
  (returns (res :type Boolean))
  ;[1 1 1] Renvoie True si le déplacement est en mode WaitOnCorners ou StopAtEnd
  (return (or (> (`self.waitOnCorners`) 0.0) (`self.stopAtEnd`))))

(fn `StepMove`
  (params (dt :type "Float (double-precision)"))
  ;[1 1 1] Gère le déplacement de la Plateforme dans le temps suivant ses settings.
  (bind _mustwait (`self.DoWaitStep` dt)) ; On gère CurrentWait et on attend encore si besoin.
  (if _mustwait
    (return) ; On doit attendre encore, on ne fait rien.
    (else
      (`self.DoStepTime` dt)
      (bind _res (`self.IsWaitOrStop`)) ; Détermine si la Plateforme boucle sans pause ou non.
      (if _res
        (`self.SubStepStop`) ; Fait des allers retours avec pause ou arrêt
        (else
          (`self.SubStepLoop`) ; Fait des allers retours sans pause ou arrêt.
        ))
      (return))))

(fn `SubStepLoop`
  ;[1 1 1] Cette fonction gère tmpTime au niveau des extrémités. Si tmpTime passe sous 0 ou au dessus 1, on change la direction de la plateforme.
  (if (> (`self.tmpTime`) 1.0)
    (set `self.tmpTime` (- 2.0 (`self.tmpTime`))) ; Si tmpTime dépasse 1, on ne doit pas tronquer bêtement à 1 sinon on perd quelques pixels de déplacement, ce qui peut poser problème si plusieurs plateformes doivent être synchronisées.
    (set `self.moveDirection` -1.0)
    (elif (< (`self.tmpTime`) 0.0)
      (set `self.tmpTime` (* (`self.tmpTime`) -1.0)) ; Pareil qu'au dessus, mais si on passe sous 0 cette fois.
      (set `self.moveDirection` 1.0)))
  (return))

(fn `SubStepStop`
  ;[1 1 1] Si tmpTime passe sous 0 ou au dessus de 1, il faut changer la direction de déplacement et soit stopper le mouvement de la Plateforme, soit le mettre en pause quelques secondes.
  (set `self.tmpTime` (`KismetMathLibrary.FClamp` (`self.tmpTime`))) ; Contrairement à SubStepLoop, on se permet de tronquer à 0 et 1 cette fois-ci, afin que la plateforme atteigne bien la position exacte des extrémités lorsqu'elle est stoppée ou mise en pause.
  (if (or (and (== (`self.tmpTime`) 0.0) (== (`self.moveDirection`) -1.0)) (and (== (`self.tmpTime`) 1.0) (== (`self.moveDirection`) 1.0)))
    (set `self.moveDirection` (* (`self.moveDirection`) -1.0))
    (if (`self.stopAtEnd`)
      (set `self.stopped` true)
      (else
        (set `self.currentWait` (`self.waitOnCorners`)))))
  (return))

(fn `UserConstructionScript`)