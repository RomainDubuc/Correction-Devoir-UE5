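; BP_Collectible_Inv is a floating pickup that grants the player invincibility.
; Tick accumulates time and offsets the Sphere component along Z by a small cosine step, producing a bobbing motion that is not scaled by frame time.
; When a BP_MyPlayer overlaps it, it calls StartInvincibility on that player, spawns a scaled-down explosion particle effect at its location and destroys itself.
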(event `self.ReceiveTick`
  (params (DeltaSeconds :type "Float (single-precision)"))
  ;[1 1 1] Ajout d'un effet de flotaison sur le Collectible
  (bind _output_get (set `self.totalTime` (+ DeltaSeconds (`self.totalTime`))))
  (`SceneComponent.K2_AddLocalOffset` (`self.Sphere`) (`KismetMathLibrary.MakeVector` 0.0 0.0 (* (`KismetMathLibrary.Cos` _output_get) 0.1)) false false))

(event `self.ReceiveActorBeginOverlap`
  (params (OtherActor :type "Actor Object Reference"))
  ;[1 1 1] Déclenche l'Invincibilité du Joueur
  (bind _asbp_my_player (cast `/Game/MyContent/Actors/BP_MyPlayer` OtherActor))
  (`/Game/MyContent/Actors/BP_MyPlayer.StartInvincibility` _asbp_my_player)
  (bind _returnvalue (`GameplayStatics.SpawnEmitterAtLocation` "/Game/StarterContent/Particles/P_Explosion.P_Explosion" (`self.K2_GetActorLocation`)))
  (`SceneComponent.SetRelativeScale3D` _returnvalue (0.1 0.0 0.1))
  (`self.K2_DestroyActor`))

(fn `UserConstructionScript`)